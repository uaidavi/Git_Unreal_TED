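; Game instance Blueprint that manages menu screens and multiplayer session hosting, joining and destruction for the arena game.
; A state-transition macro rejects repeated states, clears widgets or destroys the session on leaving a state, then lets events show lazily created, cached widgets.
; Hosting creates a two-connection session with optional LAN and opens the level; failure routes to an error screen.
; Join failure only prints a message, and the loading-screen event is empty.
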(event Custom|Loading%20Screen)

(event Custom|Show%20Server%20List
  ;[1 1 1] Abre o menu de servers
  (Utilities|StateTrans "NewEnumerator6"
    (:New%20STate
      (Utilities|IsValid (Variables|Default|GetServerList)
        (:Is%20Valid
          _)
        (:Is%20Not%20Valid
          (bind _returnvalue (UserInterface|CreateWidget "/Game/Arena_Project/Blueprints/Multiplayer/Widgets/Servers.Servers_C" (Game|GetPlayerController 0)))
          (bind _output_get (Variables|Default|SetServerList _returnvalue))))
      (UserInterface|Viewport|AddtoViewport _output_get 0)
      (Input|SetInputModeUIOnly (Game|GetPlayerController 0) _output_get false))))

(event Custom|DestroySession
  ;[1 1 1] destrui sessão
  (|DestroySession (Game|GetPlayerController 0)))

(event Custom|HostGame
  ;[1 1 1] Cria o server e vai para o nivel 1
  (|Session (Game|GetPlayerController 0) 2 (Variables|Default|GetEnableLAN)
    (:OnSuccess
      (Game|OpenLevel(byName) "Nivel_01v3" true "listen"))
    (:OnFailure
      (Utilities|DisplayError "Erro: Não foi possivel criar  a sessão"))))

(event Custom|JoinFromServerListEvent
  (params (SearchResult :type Blueprint%20Session%20Result%20Structure))
  ;[1 1 1] ENTRA NA SESSAO DO OUTRO PLAYER
  (|JoinSession (Game|GetPlayerController 0) SearchResult
    (:OnFailure
      (Development|PrintString "deu ruim"))))

(event Custom|ShowMainMenu
  ;[1 1 1] Abre o Menu
  (Utilities|IsCurrentState "NewEnumerator3"
    (:True
      (Game|OpenLevel(byName) "Main_Menu"))
    (:False
      (Utilities|StateTrans "NewEnumerator0"
        (:New%20STate
          (Utilities|IsValid (Variables|Default|GetMainMenu)
            (:Is%20Valid
              _)
            (:Is%20Not%20Valid
              (bind _returnvalue (UserInterface|CreateWidget "/Game/Arena_Project/Blueprints/Multiplayer/Widgets/Main_Menu_Widget.Main_Menu_Widget_C" (Game|GetPlayerController 0)))
              (bind _output_get (Variables|Default|SetMainMenu _returnvalue))))
          (Input|SetInputModeUIOnly (Game|GetPlayerController 0) _output_get false)
          (UserInterface|Viewport|AddtoViewport (Variables|Default|GetMainMenu) 0))))))

(fn HideWidget
  (params (widget :type Widget%20Object%20Reference))
  ;[1 1 1] destroi a widget
  (Viewport|RemoveAllWidgets))