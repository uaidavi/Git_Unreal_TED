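; Game instance Blueprint that drives the multiplayer menu flow and handles hosting and joining sessions.
; A state machine macro switches between startup, main menu, server list and arena, removing the outgoing widget, though it has no case for leaving Arena.
; Menu events lazily create and show their widgets with UI-only input.
; Hosting creates an optionally LAN session and opens the arena level, while joining uses the selected search result.
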(event Custom|Join%20From%20Server%20List
  (params (search%20result :type Blueprint%20Session%20Result%20Structure))
  ;[1 1 1] Conecta no Server[
  (|JoinSession (Game|GetPlayerController 0) search%20result
    (:OnSuccess
      (Development|PrintString "CONECTEI" true true "(R=0.143934,G=1.000000,B=0.055701,A=1.000000)" 5.0))
    (:OnFailure
      (Development|PrintString "NÃO CONSEGUIU CONECTAR"))))

(event Custom|Show%20Main_Menu
  (bind _returnvalue (Game|GetPlayerController 0))
  (Utilities|IsCurrentState "NewEnumerator3"
    (:True
      ;[1 1 1] Comment
      (Game|OpenLevel(byName) "Main_Menu"))
    (:False
      _))
  (Utilities|StateTransition "NewEnumerator0"
    (:New_State
      (Utilities|IsValid (Variables|Default|GetMain%20Menu)
        (:Is%20Valid
          _)
        (:Is%20Not%20Valid
          (bind _returnvalue_2 (UserInterface|CreateWidget "/Game/Arena_Project/Blueprints/Multiplayer/Widgets/Main_Menu_Widget.Main_Menu_Widget_C" _returnvalue))
          (bind _output_get (Variables|Default|SetMain%20Menu _returnvalue_2))))
      (Input|SetInputModeUIOnly _returnvalue _output_get false)
      (UserInterface|Viewport|AddtoViewport _output_get 0))))

(event Custom|Show%20Server%20List
  (bind _returnvalue (Game|GetPlayerController 0))
  ;[1 1 1] Mostra a lista de servers
  (Utilities|StateTransition "NewEnumerator6"
    (:New_State
      (Utilities|IsValid (Variables|Default|GetServer%20List)
        (:Is%20Valid
          _)
        (:Is%20Not%20Valid
          (bind _returnvalue_2 (UserInterface|CreateWidget "/Game/Arena_Project/Blueprints/Multiplayer/Widgets/Servers.Servers_C" _returnvalue))
          (bind _output_get (Variables|Default|SetServer%20List _returnvalue_2))))
      (UserInterface|Viewport|AddtoViewport _output_get 0)
      (Input|SetInputModeUIOnly _returnvalue _output_get false))))

(event Custom|HostGame
  ;[1 1 1] hosteia o jogo
  (|Session (Game|GetPlayerController 0) 4 (Variables|Default|GetEnableLAN)
    (:OnSuccess
      (Development|PrintString "Criei jogo")
      (Game|OpenLevel(byName) "Nivel_01v3" true "listen"))
    (:OnFailure
      (Development|PrintString "NAO DEVERIA CHEGAR AQUI" true true "(R=1.000000,G=0.042729,B=0.000000,A=1.000000)" 9.0))))

(fn StartPlayingState
  (Utilities|StateTransition "NewEnumerator3"))