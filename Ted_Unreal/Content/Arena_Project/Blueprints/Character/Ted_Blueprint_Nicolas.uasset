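; Ted character Blueprint for an arena game, handling his weak and strong melee attacks.
; Input checks stamina and attack flags, then routes through custom events into Ted_Atk, which triggers the animation Blueprint's attack flags.
; The weak attack applies authority-only damage to characters overlapping MeleeCol; the strong attack applies none here.
; Both spend stamina and use press-time checks and delays to manage cooldown flags.
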(event Custom|TED_Atk2
  (params (Atk :type Integer))
  ;[1 1 1] Ativação do ataque fraco do Ted
  (Utilities|TedAtk Atk))

(event Custom|TED_Atk3
  (params (Atk :type Integer))
  ;[1 1 1] Ativação do ataque forte do Ted
  (Utilities|TedAtk Atk))

(event EventBeginPlay
  (|CallParentFunction))

(event Collision|EventActorBeginOverlap
  (params (OtherActor :type Actor%20Object%20Reference)))

(event EventTick
  (params (DeltaSeconds :type Float%20%28single-precision%29))
  (|CallParentFunction 0.0))

(event Input|ActionEvents|InputActionAtk_2_Inp
  (params (Key :type Key%20Structure :default "AnyKey"))
  ;[1 1 1] Ativação do ataque forte do Ted
  (:Pressed
    (if (and (>= (Variables|Default|GetStamina_A) 3e+01) (Variables|Default|GetCan_Atk))
      (CallFunction|TEDAtk3 2)))
  (:Released
    (Variables|Default|SetCan_Atk true)))

(event Input|ActionEvents|InputActionAtk_1_Inp
  (params (Key :type Key%20Structure :default "AnyKey"))
  ;[1 1 1] Ativação do ataque fraco do Ted
  (:Pressed
    (if (and (and (>= (Variables|Default|GetStamina_A) 2e+01) (Variables|Default|GetCan_Atk)) (not (Variables|Default|GetInUse)))
      (Variables|Default|SetInUse true)
      (CallFunction|TEDAtk2 1)))
  (:Released
    ;;[1 1 1] Testes
    (Variables|Default|SetCan_Atk true)))

(fn ConstructionScript
  (|CallParentFunction)
  (Variables|Default|SetJust_Atked false)
  (Variables|Default|SetCan_Atk true)
  (Variables|Default|SetInUse false))