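; JumpPad is an arena actor that launches any Character overlapping it straight up with a strong, fixed vertical velocity.
; On overlap it first calls AtivacaoJumpPad on every Ted_Blueprint_Nicolas whose location nearly exactly matches the pad's own.
; It then launches the overlapping Character, overriding only vertical velocity, and sets N to 1 if that Character is a Ted_Blueprint_Nicolas.
; An unconnected Personagem_Generico_BP2 cast remains and never runs.
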(event EventBeginPlay)

(event EventActorBeginOverlap
  (params (OtherActor :type Actor%20Object%20Reference)))

(event Collision|EventActorBeginOverlap
  (params (OtherActor :type Actor%20Object%20Reference))
  (bind _outactors (Actor|GetAllActorsOfClass "/Game/Arena_Project/Blueprints/Character/Ted_Blueprint_Nicolas.Ted_Blueprint_Nicolas_C"))
  (for _array_element _outactors
    (if (Math|Vector|Equal(Vector) (Transformation|GetActorLocation) (Transformation|GetActorLocation _array_element) 0.0001)
      (Default|AtivacaoJumpPad _array_element)))
  (bind _ascharacter (Utilities|Casting|CastToCharacter OtherActor))
  (bind _asted_blueprint_nicolas (Utilities|Casting|CastToTed_Blueprint_Nicolas OtherActor)
    (:then
      (Character|LaunchCharacter _ascharacter "0.000000, 0,5000.000000" false true)
      (Variables|/Game/Arena_Project/Blueprints/Character/Personagem_Generico_BP2.Personagem_Generico_BP2_C|SetN _asted_blueprint_nicolas 1))
    (:CastFailed
      (Character|LaunchCharacter _ascharacter "0, 0,5000.000000" false true))))

(event EventTick
  (params (DeltaSeconds :type Float%20%28single-precision%29)))

(fn ConstructionScript)